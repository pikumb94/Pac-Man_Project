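; Power cell that gives the GridPawn a temporary grid-velocity boost when IA_Move both starts and completes within a precision radius of its center.
; While the cell is ready and overlapped, Tick uses normalized XY player distance to shrink and brighten a dynamic-material halo toward the center.
; Activation dims the halo, multiplies velocity for PowerupDuration, resets it, then waits the same duration again before rearming.
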(event `self.ReceiveTick`
  (params (DeltaSeconds :type "Float (single-precision)"))
  (if (`self.PowerupCooldownElapsed`)
    (if (`self.IsOverlappingWithPlayer`)
      (`self.UpdateAppearence` (`KismetMathLibrary.FClamp` (/ (`KismetMathLibrary.VSizeXY` (- (`self.K2_GetActorLocation` (`self.PlayerPawn`)) (`self.K2_GetActorLocation`))) (`SphereComponent.GetUnscaledSphereRadius` (`self.Sphere`))))))))

(event `self.ReceiveBeginPlay`
  (bind _returnvalue (`GameplayStatics.GetPlayerPawn` 0))
  (bind _simplehalo (`self.SimpleHalo`))
  (set `self.PlayerPawn` _returnvalue)
  (bind _asplayer_controller (cast `PlayerController` (`Pawn.GetController` _returnvalue)))
  (`self.EnableInput` _asplayer_controller)
  (bind _returnvalue_2 (`PrimitiveComponent.CreateDynamicMaterialInstance` _simplehalo 0 "/Game/Materials/HaloMaterial.HaloMaterial" "None"))
  (`PrimitiveComponent.SetMaterial` _simplehalo 0 _returnvalue_2)
  (set `self.HaloMaterial` _returnvalue_2))

(event `self.Sphere.OnComponentBeginOverlap`
  (params (OverlappedComponent :type "PrimitiveComponent Object Reference") (OtherActor :type "Actor Object Reference") (OtherComp :type "PrimitiveComponent Object Reference") (OtherBodyIndex :type Integer) (bFromSweep :type Boolean) (SweepResult :type "HitResult Structure (by ref)"))
  (set `self.IsOverlappingWithPlayer` true))

(event `EnhancedInput|/Game/Input/IA_Move`
  (params (ActionValue :type "Vector2D Structure") (ElapsedSeconds :type "Float (double-precision)") (TriggeredSeconds :type "Float (double-precision)") (InputAction :type "InputAction Object Reference" :default "/Game/Input/IA_Move.IA_Move"))
  (bind _halomaterial (`self.HaloMaterial`))
  (bind _powerupduration (`self.PowerupDuration`))
  (bind _returnvalue (< (`KismetMathLibrary.FClamp` (/ (`KismetMathLibrary.VSizeXY` (- (`self.K2_GetActorLocation` (`self.PlayerPawn`)) (`self.K2_GetActorLocation`))) (`SphereComponent.GetUnscaledSphereRadius` (`self.Sphere`)))) (`self.PrecisionRadiusNormalized`)))
  (:`Started`
    (if _returnvalue
      (set `self.WaitForPreciseRelease` true)
      (else
        (set `self.WaitForPreciseRelease` false))))
  (:`Completed`
    (if (`self.PowerupCooldownElapsed`)
      (if _returnvalue
        (if (`self.WaitForPreciseRelease`)
          (`KismetSystemLibrary.PrintString` "ATTIVA ABILITà!!!")
          (set `self.PowerupCooldownElapsed` false)
          (set `self.WaitForPreciseRelease` false)
          (bind _asgrid_pawn (cast `GridPawn` (`self.PlayerPawn`)))
          (bind _returnvalue_2 (`GridPawn.GetGridVelocity` _asgrid_pawn))
          (`GridPawn.SetGridVelocity` _asgrid_pawn (* _returnvalue_2 (`self.PowerupVelocityMultiplier`)))
          (`MaterialInstanceDynamic.SetScalarParameterValue` _halomaterial "Opacity" 0.0)
          (`KismetSystemLibrary.Delay` _powerupduration)
          (`GridPawn.ResetGridVelocity` _asgrid_pawn)
          (`KismetSystemLibrary.Delay` _powerupduration)
          (`MaterialInstanceDynamic.SetScalarParameterValue` _halomaterial "Opacity" 0.1)
          (set `self.PowerupCooldownElapsed` true)
          (`self.UpdateAppearence` 1.0)
          (else
            (set `self.WaitForPreciseRelease` false :!label _label)))
        (else
          (goto _label)))
      (else
        (goto _label)))))

(event `self.Sphere.OnComponentEndOverlap`
  (params (OverlappedComponent :type "PrimitiveComponent Object Reference") (OtherActor :type "Actor Object Reference") (OtherComp :type "PrimitiveComponent Object Reference") (OtherBodyIndex :type Integer))
  (set `self.IsOverlappingWithPlayer` false))

(fn `UpdateAppearence`
  (params (ClosePercentage :type "Float (double-precision)"))
  (`SceneComponent.SetWorldScale3D` (`self.SimpleHalo`) (* (`KismetMathLibrary.Lerp` 1.0 4.0 ClosePercentage) (`KismetMathLibrary.Vector_One`)))
  (`MaterialInstanceDynamic.SetScalarParameterValue` (`self.HaloMaterial`) "Opacity" (`KismetMathLibrary.Lerp` 1.0 0.25 ClosePercentage)))

(fn `UserConstructionScript`)